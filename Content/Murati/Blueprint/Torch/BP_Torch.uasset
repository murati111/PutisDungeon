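; A torch actor that can be picked up and dropped, with a fire effect and point light driven by a timeline.
; PickUp disables physics and capsule collision, attaches the torch to the given component, and plays the timeline, whose values pass through StandingFPS before setting fire scale and light intensity.
; Drop detaches it and restores physics and collision.
; Tick destroys a dropped torch after 25 seconds or once the timeline has finished.
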(event EventBeginPlay)

(event Collision|EventActorBeginOverlap
  (params (OtherActor :type Actor%20Object%20Reference)))

(event EventPickUp
  (params (AttachTo :type Scene%20Component%20Object%20Reference) (SocketName :type Name :default "None"))
  (Variables|Default|SetbDropping false)
  (Physics|SetSimulatePhysics (Variables|Default|GetStaticMesh1) false)
  (Collision|SetCollisionEnabled (Variables|Default|GetCapsule) "NoCollision")
  (Transformation|AttachComponentToComponent (VehicleSound|GetRootComponent) AttachTo "None" "KeepRelative" "KeepRelative" "KeepWorld" false)
  (Transformation|SetRelativeLocationAndRotation (Variables|Default|GetStaticMesh1) "0, 0, 0" "0, 0, 0" false false)
  (Transformation|AddActorLocalRotation (Variables|Default|GetRotation) false false)
  (Transformation|AddActorLocalOffset "0.000000,-2.000000, 0" false false)
  (bind _新規track_0 (Timeline|タイムライン_0 Play)
    (:Update
      (Transformation|SetRelativeScale3D (Variables|Default|GetP_Fire) (Math|Conversions|ToVector(Float) (* (CallFunction|StandingFPS 6e+01 _新規track_0) 2.2)))
      (Rendering|Components|Light|SetIntensity (Variables|Default|GetPointLight) (* (CallFunction|StandingFPS 6e+01 _新規track_0) 1.7e+03)))
    (:Finished
      (Variables|Default|SetbFinishFire true))))

(event EventTick
  (params (DeltaSeconds :type Float%20%28single-precision%29))
  (if (or (and (Variables|Default|GetbDropping) (>= (Math|Timespan|GetSeconds (- (Math|DateTime|Now) (Variables|Default|GetDropStartTime))) 25)) (and (Variables|Default|GetbDropping) (Variables|Default|GetbFinishFire)))
    (Actor|DestroyActor)))

(event EventDrop
  (Physics|SetSimulatePhysics (Variables|Default|GetStaticMesh1) true)
  (Collision|SetCollisionEnabled (Variables|Default|GetCapsule) "QueryAndPhysics")
  (Transformation|DetachFromActor "KeepRelative" "KeepRelative" "KeepRelative")
  (Variables|Default|SetbDropping true)
  (Variables|Default|SetDropStartTime (Math|DateTime|Now)))

(fn ConstructionScript)