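; BP_Enemy is an enemy Blueprint that supplies patrol destinations from a list of patrol points.
; GetNextPatrolPoint returns the point at the current index, then advances the index and wraps it to zero at the end, so the route loops.
; An empty list returns no point assignment, and the event graph and construction script hold no active logic.
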(event EventBeginPlay)

(event Collision|EventActorBeginOverlap
  (params (OtherActor :type Actor%20Object%20Reference)))

(event EventTick
  (params (DeltaSeconds :type Float%20%28single-precision%29)))

(fn ConstructionScript)

(fn GetNextPatrolPoint
  (if (!= (Utilities|Array|Length (Variables|Default|GetPartolPoint)) 0)
    (LocalVariables|SetNextPatrolPoint (Utilities|Array|Get(acopy) (Variables|Default|GetPartolPoint) (Variables|Default|GetPatrolPointIndex)))
    (bind _output_get (Variables|Default|SetPatrolPointIndex (+ (Variables|Default|GetPatrolPointIndex) 1)))
    (if (< _output_get (Utilities|Array|Length (Variables|Default|GetPartolPoint)))
      _
      (else
        (Variables|Default|SetPatrolPointIndex 0)))
    (return (LocalVariables|GetNextPatrolPoint))
    (else
      (return 0))))