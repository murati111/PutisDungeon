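; Player pawn BP_ClientPlayer, with axis-driven look and strafing plus an unfinished touch-drag experiment.
; Turn and LookUp feed controller yaw and pitch, MoveRight moves along the right vector, and MoveForward is empty.
; A Touch1 press stores the screen position, then Tick prints the swapped-axis drag delta as debug text without moving the pawn.
; Disconnected nodes hold touch-event enabling and moving the actor to the point under the finger.
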(event EventBeginPlay)

(event Collision|EventActorBeginOverlap
  (params (OtherActor :type Actor%20Object%20Reference)))

(event EventTick
  (params (DeltaSeconds :type Float%20%28single-precision%29))
  (bind _returnvalue (Game|GetPlayerController 0))
  (bind (_locationx _locationy _biscurrentlypressed) (Class|PlayerController|GetInputTouchState _returnvalue "Touch1"))
  (if _biscurrentlypressed
    (Variables|Default|SetNewTouchLocation (Math|Vector2D|MakeVector2D _locationx _locationy))
    (Development|PrintString (Utilities|String|Append (Utilities|String|ToString(Float) (.Y (Math|Vector2D|BreakVector2D (- (Variables|Default|GetNewTouchLocation) (Variables|Default|GetPreviousTouchLocation))))) "        " (Utilities|String|ToString(Float) (* (.X (Math|Vector2D|BreakVector2D (- (Variables|Default|GetNewTouchLocation) (Variables|Default|GetPreviousTouchLocation)))) -1.0))))
    (Variables|Default|SetPreviousTouchLocation (Variables|Default|GetNewTouchLocation))))

(event Input|AxisEvents|InputAxisTurn
  (params (AxisValue :type Float%20%28single-precision%29))
  (Pawn|Input|AddControllerYawInput AxisValue))

(event Input|AxisEvents|InputAxisLookUp
  (params (AxisValue :type Float%20%28single-precision%29))
  (Pawn|Input|AddControllerPitchInput AxisValue))

(event Input|AxisEvents|InputAxisMoveForward
  (params (AxisValue :type Float%20%28single-precision%29)))

(event Input|AxisEvents|InputAxisMoveRight
  (params (AxisValue :type Float%20%28single-precision%29))
  (Pawn|Input|AddMovementInput (Transformation|GetActorRightVector) AxisValue false))

(event Input|KeyboardEvents|W
  (params (Key :type Key%20Structure)))

(event Input|KeyboardEvents|S
  (params (Key :type Key%20Structure)))

(event Input|TouchEvents|InputTouch
  (params (Location :type Vector) (FingerIndex :type ETouchIndex%20Enum))
  (bind _returnvalue (Game|GetPlayerController 0))
  (bind (_locationx _locationy) (Class|PlayerController|GetInputTouchState _returnvalue "Touch1"))
  (:Pressed
    (if (Utilities|Enum|Equal(Enum) FingerIndex "Touch1")
      (Variables|Default|SetPreviousTouchLocation (Math|Vector2D|MakeVector2D _locationx _locationy)))))

(fn ConstructionScript)