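; Game mode Blueprint that assigns existing player characters to controllers when its OnRestartPlayer event runs.
; FindingSpawnCharacter searches the world for BP_Player and BP_ClientPlayer actors, destroys BP_Player instances after the first, and stores server and client character references.
; OnRestartPlayer then unpossesses the controller and has it possess the server character if it is local, otherwise the client character.
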(event Custom|FindingSpawnCharacter
  (bind _outactors (Actor|GetAllActorsOfClass "/Game/Murati/Blueprint/Character/BP_Player.BP_Player_C"))
  (for (_array_element _array_index) _outactors
    (if (== _array_index 0)
      (Utilities|IsValid _array_element
        (:Is%20Valid
          (Utilities|FlowControl|Delay 0.0)))
      (else
        (Actor|DestroyActor _array_element))))
  (Variables|Default|SetServerCharacter _array_element)
  (bind _outactors_2 (Actor|GetAllActorsOfClass "/Game/Murati/Blueprint/Character/BP_ClientPlayer.BP_ClientPlayer_C"))
  (for _array_element_2 _outactors_2
    (Utilities|IsValid _array_element_2
      (:Is%20Valid
        (Utilities|FlowControl|Delay 0.0))))
  (Variables|Default|SetClientCharacter _array_element_2))

(event EventBeginPlay)

(event EventTick
  (params (DeltaSeconds :type Float%20%28single-precision%29)))

(event EventOnRestartPlayer
  (params (NewPlayer :type Controller%20Object%20Reference))
  (CallFunction|FindingSpawnCharacter)
  (Pawn|UnPossess NewPlayer)
  (if (Pawn|IsLocalPlayerController NewPlayer)
    (Pawn|Possess NewPlayer (Variables|Default|GetServerCharacter))
    (else
      (Pawn|Possess NewPlayer (Variables|Default|GetClientCharacter)))))

(fn ConstructionScript)