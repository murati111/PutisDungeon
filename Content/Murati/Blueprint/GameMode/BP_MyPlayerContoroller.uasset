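; Player controller that turns single-finger touch drags into world-space movement of its own actor.
; Pressing Touch1 records the start location, then each tick while held applies the screen delta as an unswept world offset.
; Screen vertical motion maps to world X and inverted horizontal motion to world Y, with no scaling.
; An unconnected leftover branch that nudges a BP_ClientPlayer pawn never runs.
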(event EventBeginPlay)

(event EventTick
  (params (DeltaSeconds :type Float%20%28single-precision%29))
  (bind (_locationx _locationy _biscurrentlypressed) (Class|PlayerController|GetInputTouchState "Touch1"))
  (if _biscurrentlypressed
    (Variables|Default|SetNewTouchLocation (Math|Vector2D|MakeVector2D _locationx _locationy))
    (Transformation|AddActorWorldOffset (Math|Vector|MakeVector (.Y (Math|Vector2D|BreakVector2D (- (Variables|Default|GetNewTouchLocation) (Variables|Default|GetPreviousTouchLocation)))) (* (.X (Math|Vector2D|BreakVector2D (- (Variables|Default|GetNewTouchLocation) (Variables|Default|GetPreviousTouchLocation)))) -1.0) 0.0))
    (Variables|Default|SetPreviousTouchLocation (Variables|Default|GetNewTouchLocation))))

(event Input|KeyboardEvents|W
  (params (Key :type Key%20Structure)))

(event Input|TouchEvents|InputTouch
  (params (Location :type Vector) (FingerIndex :type ETouchIndex%20Enum))
  (bind (_locationx _locationy) (Class|PlayerController|GetInputTouchState "Touch1"))
  (:Pressed
    (if (Utilities|Enum|Equal(Enum) FingerIndex "Touch1")
      (Variables|Default|SetPreviousTouchLocation (Math|Vector2D|MakeVector2D _locationx _locationy)))))

(fn ConstructionScript)