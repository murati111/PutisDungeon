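; BP_MyPlayerState is a player state Blueprint declaring pick-up and drop events for torches, but both event bodies are empty.
; Disconnected, never-executed nodes hold attach and detach logic that toggles torch mesh physics and capsule collision.
; The unused pick-up chain also plays a timeline that scales the torch's fire effect and point light intensity.
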(event Custom|PickUpAction
  (params (BP_Torch :type BP%20Torch%20Object%20Reference) (Parent :type Scene%20Component%20Object%20Reference)))

(event Custom|DropAction
  (params (NewParam :type BP%20Torch%20Object%20Reference)))

(event EventBeginPlay)

(event EventTick
  (params (DeltaSeconds :type Float%20%28single-precision%29)))

(fn ConstructionScript)