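; BP_MyGameinstance is a game instance that hosts and joins online multiplayer sessions.
; HostSession creates a session with the given LAN flag and connection count, then opens the first stage as a listen server on success.
; JoinSession joins a supplied search result for the first player controller, and both events print their success or failure.
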(event Custom|JoinSession
  (params (SessionToJoin :type Blueprint%20Session%20Result%20Structure%20%28by%20ref%29))
  ;[1 1 1] セッションに参加
  (|JoinSession (Game|GetPlayerController 0) SessionToJoin
    (:OnSuccess
      (Development|PrintString "JoinSession:Sucess"))
    (:OnFailure
      (Development|PrintString "JoinSession:Failed"))))

(event Custom|HostSession
  (params (bUseLAN :type Boolean) (PublicConnections :type Integer))
  ;[1 1 1] セッションを作成
  (|Session (Game|GetPlayerController 0) PublicConnections bUseLAN
    (:OnSuccess
      (Development|PrintString "CreateSession:Sucess")
      (Game|OpenLevel(byName) (Variables|Default|GetFirstStageName) true "listen"))
    (:OnFailure
      (Development|PrintString "CreateSession:Failed"))))