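; Work-in-progress interactive door that swings in yaw in response to a vector value passed through its Interacting event.
; MoveDoor adds the Arrow's forward X to door yaw when the input nearly matches that forward vector, with debug prints.
; Hover, sphere-overlap player proximity and a once-cached handle position are stored but do not affect movement.
; The angle-between-vectors helper and camera-based calculations are disconnected, and CalculateAndReport and InitSlider are empty.
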(event OnComponentBeginOverlap(Sphere)
  (params (OverlappedComponent :type Primitive%20Component%20Object%20Reference) (OtherActor :type Actor%20Object%20Reference) (OtherComp :type Primitive%20Component%20Object%20Reference) (OtherBodyIndex :type Integer) (bFromSweep :type Boolean) (SweepResult :type Hit%20Result%20Structure%20%28by%20ref%29))
  (bind _returnvalue (Actor|ActorHasTag OtherActor "Player"))
  (Development|PrintString (Utilities|String|ToString(Boolean) _returnvalue))
  (Variables|Default|SetbIsNearPlayer _returnvalue))

(event EventBeginPlay)

(event Collision|EventActorBeginOverlap
  (params (OtherActor :type Actor%20Object%20Reference)))

(event EventTick
  (params (DeltaSeconds :type Float%20%28single-precision%29)))

(event EventBeginHover
  (Variables|Default|SetIsHovering true))

(event EventEndHover
  (Variables|Default|SetIsHovering false))

(event EventInteracting
  (params (MouceValue :type Vector :default "0, 0, 0"))
  (bind _boxhandle (Variables|Default|GetBoxHandle))
  (bind _returnvalue (Transformation|GetWorldLocation _boxhandle))
  (bind (_x _y) (Math|Vector|BreakVector _returnvalue))
  (CallFunction|MoveDoor MouceValue)
  (Utilities|FlowControl|DoOnce false
    (:Completed
      (Variables|Default|SetHandleVector (Math|Vector|MakeVector _x _y (.Z (Math|Vector|BreakVector (Transformation|GetWorldLocation (Variables|Default|GetDoor)))))))))

(fn ConstructionScript)

(fn MoveDoor
  (params (NewParam :type Vector))
  (bind _door (Variables|Default|GetDoor))
  (bind _arrow (Variables|Default|GetArrow))
  (bind _returnvalue (Math|Vector|GetForwardVector _arrow))
  (bind _relativerotation (Variables|/Script/Engine.SceneComponent|GetRelativeRotation _door))
  (bind (_roll _pitch _yaw) (Math|Rotator|BreakRotator _relativerotation))
  (Development|PrintString (Utilities|String|Append (Utilities|String|ToString(Vector) NewParam) "   " (Utilities|String|ToString(Vector) _returnvalue)))
  (if (Math|Vector|Equal(Vector) NewParam _returnvalue 0.5)
    (Development|PrintString "Hello")
    (Transformation|SetRelativeRotation _door (Math|Rotator|MakeRotator _roll _pitch (+ _yaw (.X (Math|Vector|BreakVector _returnvalue)))) false false)))

(fn CalculateandReport)

(fn InitSlider)

(fn MakeAnglefrom2Vectors
  (params (AxisPoint :type Vector) (FirstPoint :type Vector) (SecondPoint :type Vector))
  (bind _returnvalue (- SecondPoint AxisPoint))
  (bind _returnvalue_2 (- FirstPoint AxisPoint))
  (return (Class|KismetMathLibrary|DegAcos (/ (Math|Vector|DotProduct _returnvalue _returnvalue_2) (* (Math|Vector|VectorLength _returnvalue_2) (Math|Vector|VectorLength _returnvalue)))) (.z (* _returnvalue _returnvalue_2))))